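; BP_LORELibrary is a library of tabletop RPG-style helper functions for dice rolls and ability score bonuses.
; Separate functions roll a D4, D6, D8, D10, D12 or D20, each returning a uniform random integer.
; CalculateAbilityScoreBonus halves the score's offset from ten, with a separate branch for zero or negative scores that adds eleven before halving.
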(fn RollD4
  (return (Math|Random|RandomIntegerinRange 1 4)))

(fn RollD6
  (return (Math|Random|RandomIntegerinRange 1 6)))

(fn RollD8
  (return (Math|Random|RandomIntegerinRange 1 8)))

(fn RollD10
  (return (Math|Random|RandomIntegerinRange 1 10)))

(fn RollD12
  (return (Math|Random|RandomIntegerinRange 1 12)))

(fn RollD20
  (return (Math|Random|RandomIntegerinRange 1 20)))

(fn CalculateAbilityScoreBonus
  (params (Score :type Integer))
  (if (<= Score 0)
    (return (/ (- Score -11) 2))
    (else
      (return (/ (- Score 10) 2)))))